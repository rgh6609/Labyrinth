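; BP_ADEnemy is an enemy Blueprint that repeatedly fires at the player once its attack starts.
; StartAttack extends the parent behavior with a looping timer, which this graph never clears.
; On each tick of that timer, the enemy snaps its full rotation toward player 0's pawn and spawns a TestFire actor at its own location and rotation.
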(event `self.ReceiveBeginPlay`)

(event `self.StartAttack`
  (`parent.StartAttack`)
  (`KismetSystemLibrary.K2_SetTimerDelegate` (delegate `CustomEvent`) 1.5 true))

(event `CustomEvent`
  (`self.K2_SetActorRotation` (`KismetMathLibrary.FindLookAtRotation` (`self.K2_GetActorLocation`) (`self.K2_GetActorLocation` (`GameplayStatics.GetPlayerPawn` 0))))
  (`|SpawnActorFromClass` "/Game/Main/Enemy/Blueprints/AttackEffect/TestFire.TestFire_C" (`KismetMathLibrary.MakeTransform` (`self.K2_GetActorLocation`) (`self.K2_GetActorRotation`)) "Undefined" "MultiplyWithRoot" null null))

(fn `UserConstructionScript`)